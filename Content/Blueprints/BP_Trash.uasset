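; BP_Trash is a falling trash piece that the player's BP_Robot catches before it drops out of the level.
; Each Tick moves it down a fixed step per frame, independent of delta time.
; A first robot overlap adds score, updates the HUD and spawns a BP_BeltItem offset from the BP_Conveyor.
; Falling below the Z limit raises robot pollution on the HUD, showing the lose screen and pausing at maximum.
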(event EventBeginPlay)

(event Collision|EventActorBeginOverlap
  (params (OtherActor :type Actor%20Object%20Reference))
  (bind _asbp_robot (Utilities|Casting|CastToBP_Robot OtherActor))
  (if (not (Variables|Default|GetCaught))
    (Variables|Default|SetCaught true)
    (bind _output_get (Variables|/Game/Blueprints/BP_Robot.BP_Robot_C|SetScore _asbp_robot (+ (Variables|/Game/Blueprints/BP_Robot.BP_Robot_C|GetScore _asbp_robot) 1)))
    (Variables|/Game/UI/WBP_HUD.WBP_HUD_C|SetScore (Variables|/Game/Blueprints/BP_Robot.BP_Robot_C|GetHUD _asbp_robot) _output_get)
    (bind _returnvalue (Actor|GetActorOfClass "/Game/Blueprints/BP_Conveyor.BP_Conveyor_C"))
    (Game|SpawnActorfromClass "/Game/Blueprints/BP_BeltItem.BP_BeltItem_C" (Math|Transform|MakeTransform (+ (Transformation|GetActorLocation _returnvalue) "900.000000,-100.000000,0.000000") "0, 0, 0" "1.000000,1.000000,1.000000") "Undefined" "MultiplyWithRoot" 0 0)
    (Actor|DestroyActor)))

(event EventTick
  (params (DeltaSeconds :type Float%20%28single-precision%29))
  (Transformation|AddActorWorldOffset (Math|Vector|MakeVector 0.0 0.0 -2.0))
  (if (< (.Z (Math|Vector|BreakVector (Transformation|GetActorLocation))) -5e+02)
    (bind _asbp_robot (Utilities|Casting|CastToBP_Robot (Game|Player|GetPlayerPawn 0)))
    (bind _output_get (Variables|/Game/Blueprints/BP_Robot.BP_Robot_C|SetPollution _asbp_robot (+ (Variables|/Game/Blueprints/BP_Robot.BP_Robot_C|GetPollution _asbp_robot) 1e+01)))
    (bind _output_get_2 (Variables|/Game/UI/WBP_HUD.WBP_HUD_C|SetPollutionPercent (Variables|/Game/Blueprints/BP_Robot.BP_Robot_C|GetHUD _asbp_robot) (/ _output_get (Variables|/Game/Blueprints/BP_Robot.BP_Robot_C|GetPollutionMax _asbp_robot))))
    (if (>= _output_get_2 1.0)
      (Default|ShowLose (Variables|/Game/Blueprints/BP_Robot.BP_Robot_C|GetHUD _asbp_robot))
      (Game|SetGamePaused true))
    (Actor|DestroyActor)))

(fn ConstructionScript)